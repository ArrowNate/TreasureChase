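; Player character for a Paper2D game, with jump, crouch-based slide, pause menu, timed invincibility and death.
; Tick picks the run, slide, jump, fall or death flipbook from movement state and the death flag.
; Death, unless invincible, shows a game-over widget and pauses after a short delay.
; BeginPlay is empty; the HUD and looping distance-counter setup is disconnected, so neither starts here.
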(event Custom|Update%20Animation
  ;[1 1 1] Handle Player Animation
  (if (not (Variables|Default|GetIsDead))
    (if (AI|Components|NavMovement|IsMovingonGround (Variables|Character|GetCharacterMovement))
      (if (AI|Components|NavMovement|IsCrouching (Variables|Character|GetCharacterMovement))
        (CallFunction|UpdateFlipbook "/Game/Animations/SlidingAnimation.SlidingAnimation")
        (else
          (CallFunction|UpdateFlipbook "/Game/Animations/RunningAnimation.RunningAnimation")))
      (elif (> (.z (Transformation|GetVelocity)) 0.0)
        (CallFunction|UpdateFlipbook "/Game/Animations/JumpAnimation.JumpAnimation")
        (else
          (CallFunction|UpdateFlipbook "/Game/Animations/FallAnimation.FallAnimation"))))
    (else
      (Sprite|SetFlipbook (Variables|Default|GetSprite) "/Game/Animations/DeathAnimation.DeathAnimation"))))

(event Custom|Death
  ;[1 1 1] Player Death
  (if (not (Variables|Default|GetIsInvincible))
    (Variables|Default|SetIsDead true)
    (bind _returnvalue (UserInterface|CreateWidget "/Game/Blueprints/BP_Gameover.BP_Gameover_C"))
    (UserInterface|Viewport|AddtoViewport _returnvalue 0)
    (Utilities|FlowControl|Delay 0.5)
    (Game|SetGamePaused true)))

(event Custom|Update%20Distance
  ;[1 1 1] Event BeginPlay (In-Game HUD)
  (bind _result (Math|Integer|IncrementInt (Variables|Default|GetDistanceInteger))
    (:%20%20
      (Default|UpdateDistance (Variables|Default|GetDistance) _result))))

(event Custom|Invincible
  ;[1 1 1] Handle Player Invincibility
  (Variables|Default|SetIsInvincible true)
  (Utilities|FlowControl|Delay 1e+01)
  (Variables|Default|SetIsInvincible false))

(event EventBeginPlay
  ;[1 1 1] Event BeginPlay (In-Game HUD)
)

(event EventTick
  (params (DeltaSeconds :type Float%20%28single-precision%29))
  (CallFunction|UpdateAnimation))

(event Input|ActionEvents|InputActionJumpAction
  (params (Key :type Key%20Structure :default "None"))
  ;[1 1 1] Handle Player Jump
  (:Pressed
    (Character|Jump))
  (:Released
    (Character|StopJumping)))

(event Input|ActionEvents|InputActionSlide
  (params (Key :type Key%20Structure :default "None"))
  ;[1 1 1] Handle Player Sliding
  (:Pressed
    (Character|Crouch)
    (Transformation|SetRelativeLocation (Variables|Default|GetSprite) "0, 0,15.000000" false false))
  (:Released
    (Character|UnCrouch)
    (Transformation|SetRelativeLocation (Variables|Default|GetSprite) "0, 0, 0" false false)))

(event Input|ActionEvents|InputActionPauseGame
  (params (Key :type Key%20Structure :default "None"))
  (bind _returnvalue (Game|GetPlayerController 0))
  ;[1 1 1] Pausing and Unpausing Game
  (:Pressed
    (Utilities|IsValid 0
      (:Is%20Valid
        _)
      (:Is%20Not%20Valid
        (bind _returnvalue_2 (UserInterface|CreateWidget "/Game/Blueprints/BP_Pause.BP_Pause_C"))
        (Variables|Default|SetPause%20Menu%20Reference _returnvalue_2)))
    (if (Game|IsGamePaused)
      (Widget|RemovefromParent (Variables|Default|GetPause%20Menu%20Reference))
      (Game|SetGamePaused false)
      (Variables|/Script/Engine.PlayerController|SetbShowMouseCursor _returnvalue true)
      (Input|SetInputModeGameOnly _returnvalue)
      (else
        (UserInterface|Viewport|AddtoViewport (Variables|Default|GetPause%20Menu%20Reference) 0)
        (Game|SetGamePaused true)
        (Variables|/Script/Engine.PlayerController|SetbShowMouseCursor _returnvalue true)
        (Input|SetInputModeGameandUI _returnvalue (Variables|Default|GetPause%20Menu%20Reference) "DoNotLock" false)))))

(fn ConstructionScript)

(fn UpdateFlipbook
  (params (Flipbook%20Animation :type Paper%20Flipbook%20Object%20Reference))
  (Sprite|SetFlipbook (Variables|Default|GetSprite) Flipbook%20Animation))